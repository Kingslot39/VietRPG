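; Test main character Blueprint with a Paper2D sprite and a Left Shift dash.
; BeginDash swaps the flipbook, briefly ignores Pawn collision and lerps the actor to TeleportFoward's result on a timeline scaled by DashDuration, without sweeping.
; GetFurtherValidLocation steps capsule overlap tests back from the far end to find a landing spot free of Pawn blockers, with an upward Visibility hit required.
; Tick passes IsDash to SetIsDashing.
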(event `self.ReceiveTick`
  (params (DeltaSeconds :type "Float (single-precision)"))
  ;[1 1 1] Dash
  (`self.SetIsDashing` (`self.IsDash`)))

(event `TurnOffCollision`
  (bind _capsulecomponent (`self.CapsuleComponent`))
  ;[1 1 1] Dash
  (if (`self.IsDash`)
    (`PrimitiveComponent.SetCollisionEnabled` _capsulecomponent "NoCollision")
    (`KismetSystemLibrary.Delay` 1.0)
    (`PrimitiveComponent.SetCollisionEnabled` _capsulecomponent "QueryAndPhysics")))

(event `Key|LeftShift`
  (params (Key :type "Key Structure"))
  ;[1 1 1] Dash
  (:`Pressed`
    (`self.Begin Dash`)))

(event `Begin Dash`
  (bind _capsulecomponent (`self.CapsuleComponent`))
  ;[1 1 1] Dash
  (set `self.IsDash` true)
  (`PrimitiveComponent.SetCollisionResponseToChannel` _capsulecomponent "ECC_Pawn" "ECR_Ignore")
  (`PaperFlipbookComponent.SetFlipbook` (`self.Sprite`) "/Game/MainCharacter/Dash/Dashing2frame.Dashing2frame")
  (bind _returnvalue (`self.TeleportFoward`))
  (`self.MoveOverTime` _returnvalue)
  (`KismetSystemLibrary.Delay` 0.2)
  (`PrimitiveComponent.SetCollisionResponseToChannel` _capsulecomponent "ECC_Pawn" "ECR_Block")
  (set `self.IsDash` false))

(event `MoveOverTime`
  (params (Location :type "Vector Structure"))
  ;[1 1 1] Dash
  (set `self.DashStartLocation` (`self.K2_GetActorLocation`))
  (`TimelineComponent.SetPlayRate` (`self.DashTimeline`) (/ 1.0 (`self.DashDuration`)))
  (bind (_direction _locationalpha) (`Timeline|DashTimeline` :!via `PlayFromStart`)
    (:`Update`
      (`self.K2_SetActorLocation` (`KismetMathLibrary.VLerp` (`self.DashStartLocation`) Location _locationalpha) false true))))

(event `self.ReceiveBeginPlay`
  (`SceneComponent.SetMobility` (`self.CapsuleComponent`) "Movable"))

(fn `GetFurtherValidLocation`
  (params (Start :type "Vector Structure") (End :type "Vector Structure"))
  (returns (Location :type "Vector Structure"))
  (locals (Direction :type "Vector Structure" :default (0.0 0.0 0.0)) (CapsuleDiameter :type "Float (double-precision)") (CapsuleCount :type Integer) (CurrentCapsuleLocation :type "Vector Structure"))
  (bind (_outradius _outhalfheight) (`CapsuleComponent.GetUnscaledCapsuleSize` (`self.CapsuleComponent`)))
  (set `local.Direction` (`KismetMathLibrary.GetDirectionUnitVector` Start End))
  (bind _output_get (set `local.CapsuleDiameter` (* (`CapsuleComponent.CapsuleRadius` (`self.CapsuleComponent`)) 2.0)))
  (bind _output_get_2 (set `local.CapsuleCount` (/ (`KismetMathLibrary.Vector_Distance` Start End) _output_get)))
  (for _index (range (+ _output_get_2 1))
    (bind _returnvalue (+ (* (- (`local.CapsuleCount`) _index) (`local.Direction`) (`local.CapsuleDiameter`)) Start))
    (bind _output_get_3 (set `local.CurrentCapsuleLocation` _returnvalue))
    (bind _outhits (`KismetSystemLibrary.CapsuleTraceMultiForObjects` _returnvalue _returnvalue _outradius _outhalfheight (`|MakeArray` "ObjectTypeQuery1" :!type "EObjectTypeQuery Enum")))
    (bind _isvalid (`self.IsValidDashLocation` _output_get_3 _outhits))
    (if _isvalid
      (return (`local.CurrentCapsuleLocation`))))
  (return Start))

(fn `IsValidDashLocation`
  (params (Location :type "Vector Structure") (Hits :type "Array of HitResult Structure"))
  (returns (IsValid :type Boolean))
  (bind (_outhit _returnvalue) (`KismetSystemLibrary.LineTraceSingle` Location (+ Location (0.0 0.0 500.0)) "TraceTypeQuery1"))
  (if _returnvalue
    (if (`KismetArrayLibrary.Array_IsEmpty` Hits)
      (return true)
      (else
        (for _array_element Hits
          (if (`|EnumEquality` (`PrimitiveComponent.GetCollisionResponseToChannel` (`.HitComponent` (`GameplayStatics.BreakHitResult` _array_element)) "ECC_Pawn") "ECR_Block")
            (return false)))
        (return true)))
    (else
      (return false))))

(fn `UserConstructionScript`)